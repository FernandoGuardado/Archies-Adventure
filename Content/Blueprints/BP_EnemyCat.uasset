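; A Paper2D enemy cat that fires hairballs at the player when they come within short horizontal range.
; Tick compares sprite and player X positions, flips the sprite by rotation according to side, then calls ShootHairball.
; A DoOnce reset after a delay rate-limits hairballs, which spawn at the Arrow component's transform.
; DamageEnemyCat subtracts from health and destroys the actor at zero or below.
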(event Custom|DamageEnemyCat
  (params (DamageTaken :type Float%20%28single-precision%29))
  ;[1 1 1] Damage to cat
  (bind _output_get (Variables|Default|SetEnemyCatHealth (- (Variables|Default|GetEnemyCatHealth) DamageTaken)))
  (Math|Float|CompareFloat _output_get 0.0
    (:==
      _)
    (:<
      _))
  (Actor|DestroyActor))

(event Custom|ShootHairball
  ;[1 1 1] Cat shooting
  (Utilities|FlowControl|DoOnce false :!label _label
    (:Completed
      (Game|SpawnActorfromClass "/Game/Blueprints/BP_Hairball.BP_Hairball_C" (Transformation|GetWorldTransform (Variables|Default|GetArrow)) "Undefined" 0 0)
      (Utilities|FlowControl|Delay 2.0)
      (goto _label Reset))))

(event EventTick
  (params (DeltaSeconds :type Float%20%28single-precision%29))
  (bind _returnvalue (Game|GetPlayerCharacter 0))
  (bind _papersprite (Variables|Default|GetPaperSprite))
  (bind _returnvalue_2 (Transformation|GetWorldLocation _papersprite))
  (bind _returnvalue_3 (Transformation|GetActorLocation _returnvalue))
  (bind _returnvalue_4 (- (.x _returnvalue_2) (.x _returnvalue_3)))
  ;[1 1 1] Shoot Archie when in range
  (Utilities|FlowControl|Sequence
    (:then_0
      (if (> _returnvalue_4 0.0)
        (if (< _returnvalue_4 1.5e+02)
          (Transformation|SetRelativeRotation (Variables|Default|GetPaperSprite) "0, 0, 0" false false)
          (CallFunction|ShootHairball))))
    (:then_1
      (if (< _returnvalue_4 0.0)
        (if (> _returnvalue_4 -1.5e+02)
          (Transformation|SetRelativeRotation (Variables|Default|GetPaperSprite) "0,180.000000, 0" false false)
          (CallFunction|ShootHairball))))))

(fn ConstructionScript)